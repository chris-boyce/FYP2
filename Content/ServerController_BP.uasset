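; Server controller that persists bot stats and matchmaking records, both skill rating and TrueSkill Mu/Sigma, as CSV files in the project content directory.
; Events seed string arrays from DataTables, parse them into maps keyed by bot ID, and edit entries, usually rewriting the CSV.
; EndPlay and RefreshArray flush the skill-rating map to disk; a separate event backs up TrueSkill rows per level save.
; InGame always serializes as FALSE.
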(event `self.BotStatsWriteDataTableToArray`
  ;[0.1039 0.1866 1] Data Stats Saving and Loading and editing
  (bind _outrownames (`DataTableFunctionLibrary.GetDataTableRowNames` "/Game/BotData.BotData"))
  (for _array_element _outrownames
    (bind _returnvalue (`|GetDataTableRow` "/Game/BotData.BotData" _array_element)
      (:`then`
        (bind (_idnum _reactiontime _shotaccuracy) (break `/Game/BotDataStruct` _returnvalue))
        (bind _newparam3 (`self.BotStatsVarToString` _idnum _reactiontime _shotaccuracy))
        (`KismetArrayLibrary.Array_AddUnique` (`self.OutText`) _newparam3)
        (`TextFileManager.SaveArrayText` (`BlueprintPathsLibrary.ProjectContentDir`) "BotData.csv" (`self.OutText`) true)))))

(event `self.BotStatsWriteArrayToMap`
  ;[0.1039 0.1866 1] Data Stats Saving and Loading and editing
  (for _array_element (`self.OutText`)
    (bind (_newparam1 _newparam2 _newparam3) (`self.BotStatsStringToVars` _array_element))
    (`BlueprintMapLibrary.Map_Add` (`self.BotStatsMap`) _newparam1 (make `BotData` _newparam1 _newparam2 _newparam3))))

(event `self.BotStatsEditDataInMapAndArray`
  (params (IDNum :type Integer) (ReactionTime :type "Float (single-precision)") (Accuracy :type "Float (single-precision)"))
  ;[0.1039 0.1866 1] Data Stats Saving and Loading and editing
  (bind _newparam3 (`self.BotStatsVarToString` IDNum ReactionTime Accuracy))
  (`KismetArrayLibrary.Array_Set` (`self.OutText`) (+ IDNum 1) _newparam3)
  (`TextFileManager.SaveArrayText` (`BlueprintPathsLibrary.ProjectContentDir`) "BotData.csv" (`self.OutText`) true)
  (`BlueprintMapLibrary.Map_Add` (`self.BotStatsMap`) IDNum (make `BotData` IDNum ReactionTime Accuracy)))

(event `self.ServerWriteDataTableToArray`
  (bind _outrownames (`DataTableFunctionLibrary.GetDataTableRowNames` "/Game/ServerData.ServerData"))
  (for _array_element _outrownames
    (bind _returnvalue (`|GetDataTableRow` "/Game/ServerData.ServerData" _array_element)
      (:`then`
        (bind (_idnum _ingame _gamesplayed _skillrating) (break `BotSeverData` _returnvalue))
        (bind _outstring (`self.ServerStatsVarToString` _idnum _ingame _gamesplayed _skillrating))
        (`KismetArrayLibrary.Array_AddUnique` (`self.ServerOutText`) _outstring)
        (`TextFileManager.SaveArrayText` (`BlueprintPathsLibrary.ProjectContentDir`) "BotServerData.csv" (`self.ServerOutText`) true)))))

(event `self.ServerWriteDataTableToArrayTS`
  (bind _outrownames (`DataTableFunctionLibrary.GetDataTableRowNames` "/Game/BotDataTrueSkill.BotDataTrueSkill"))
  (for _array_element _outrownames
    (bind _returnvalue (`|GetDataTableRow` "/Game/BotDataTrueSkill.BotDataTrueSkill" _array_element)
      (:`then`
        (bind (_idnum _ingame _gamesplayed _mu _sigma) (break `BotSeverDataTrueSkill` _returnvalue))
        (bind _newparam (`self.BotStatsVarToStringTS` _idnum _ingame _gamesplayed _mu _sigma))
        (`KismetArrayLibrary.Array_AddUnique` (`self.OutTextTS`) _newparam)
        (`TextFileManager.SaveArrayText` (`BlueprintPathsLibrary.ProjectContentDir`) "BotServerDataTrueSkill.csv" (`self.OutTextTS`) true)))))

(event `self.ServerWriteArrayToMap`
  (for _array_element (`self.ServerOutText`)
    (bind (_idnum _ingame _gamesplayed _skillrating) (`self.ServerVarToString` _array_element))
    (`BlueprintMapLibrary.Map_Add` (`self.BotServerStatus`) _idnum (make `BotSeverData` _idnum _ingame _gamesplayed _skillrating))))

(event `self.ServerWriteArrayToMapTS`
  (for _array_element (`self.OutTextTS`)
    (bind (_id _gamesplayed _mu _sigma) (`self.BotStatsStringToVarsTS` _array_element))
    (`BlueprintMapLibrary.Map_Add` (`self.BotServerStatusTS`) _id (make `BotSeverDataTrueSkill` _id false _gamesplayed _mu _sigma))))

(event `self.ServerEditDataInMapAndArray`
  (params (IDNum :type Integer) (GamesPlayed :type Integer) (SkillRating :type "Float (single-precision)"))
  (bind _outstring (`self.ServerStatsVarToString` IDNum false GamesPlayed SkillRating))
  (`KismetArrayLibrary.Array_Set` (`self.ServerOutText`) (+ IDNum 1) _outstring)
  (`TextFileManager.SaveArrayText` (`BlueprintPathsLibrary.ProjectContentDir`) "BotServerData.csv" (`self.ServerOutText`) true)
  (`BlueprintMapLibrary.Map_Add` (`self.BotServerStatus`) IDNum (make `BotSeverData` IDNum false GamesPlayed SkillRating)))

(event `self.ServerEditMap`
  (params (IDNum :type Integer) (GamesPlayed :type Integer) (SkillRating :type "Float (single-precision)"))
  (`BlueprintMapLibrary.Map_Add` (`self.BotServerStatus`) IDNum (make `BotSeverData` IDNum false GamesPlayed SkillRating)))

(event `self.ServerEditDataInMapAndArrayTS`
  (params (IDNum :type Integer) (GamesPlayed :type Integer) (Mu :type "Float (single-precision)") (Sigma :type "Float (single-precision)"))
  (bind _newparam (`self.BotStatsVarToStringTS` IDNum false GamesPlayed Mu Sigma))
  (`KismetArrayLibrary.Array_Set` (`self.OutTextTS`) (+ IDNum 1) _newparam)
  (`TextFileManager.SaveArrayText` (`BlueprintPathsLibrary.ProjectContentDir`) "BotServerDataTrueSkill.csv" (`self.OutTextTS`) true)
  (`BlueprintMapLibrary.Map_Add` (`self.BotServerStatusTS`) IDNum (make `BotSeverDataTrueSkill` IDNum false GamesPlayed Mu Sigma)))

(event `self.ReceiveEndPlay`
  (params (EndPlayReason :type "EEndPlayReason Enum" :default "Destroyed"))
  (for _index (range 1 (+ (`BlueprintMapLibrary.Map_Length` (`self.BotServerStatus`)) 1)) :!label _label
    (bind (_idnum _ingame _gamesplayed _skillrating) (break `BotSeverData` (`BlueprintMapLibrary.Map_Find` (`self.BotServerStatus`) (- _index 1))))
    (bind _outstring (`self.ServerStatsVarToString` _idnum _ingame _gamesplayed _skillrating))
    (`KismetArrayLibrary.Array_Set` (`self.ServerOutText`) (+ _idnum 1) _outstring)
    (`TextFileManager.SaveArrayText` (`BlueprintPathsLibrary.ProjectContentDir`) "BotServerData.csv" (`self.ServerOutText`) true)))

(event `self.RefreshArray`
  (goto _label))

(event `self.SaveBotStatsToNewFileAtEndLevel`
  (`TextFileManager.SaveArrayText` (`KismetStringLibrary.Concat_StrStr` (`BlueprintPathsLibrary.ProjectContentDir`) "\\\\Backup") (`KismetStringLibrary.Concat_StrStr` "BackupSave" (`KismetStringLibrary.Conv_IntToString` (`self.LevelSave`)) ".csv") (`self.OutTextTS`) true))

(fn `BotStatsStringToVars`
  (params (NewParam :type String))
  (returns (NewParam1 :type Integer) (NewParam2 :type "Float (double-precision)") (NewParam3 :type "Float (double-precision)"))
  (bind _returnvalue (`KismetStringLibrary.ParseIntoArray` NewParam ","))
  (return (`KismetStringLibrary.Conv_StringToInt` (`|GetArrayItem` _returnvalue 1)) (`KismetStringLibrary.Conv_StringToDouble` (`|GetArrayItem` _returnvalue 2)) (`KismetStringLibrary.Conv_StringToDouble` (`|GetArrayItem` _returnvalue 3))))

(fn `BotStatsStringToVarsTS`
  (params (NewParam :type String))
  (returns (ID :type Integer) (GamesPlayed :type Integer) (Mu :type "Float (double-precision)") (Sigma :type "Float (double-precision)"))
  (bind _returnvalue (`KismetStringLibrary.ParseIntoArray` NewParam ","))
  (return (`KismetStringLibrary.Conv_StringToInt` (`|GetArrayItem` _returnvalue 1)) (`KismetStringLibrary.Conv_StringToInt` (`|GetArrayItem` _returnvalue 3)) (`KismetStringLibrary.Conv_StringToDouble` (`|GetArrayItem` _returnvalue 4)) (`KismetStringLibrary.Conv_StringToDouble` (`|GetArrayItem` _returnvalue 5))))

(fn `BotStatsVarToString`
  (params (IdNum :type Integer) (Mu :type "Float (double-precision)") (Sigma :type "Float (double-precision)"))
  (returns (NewParam3 :type String))
  (return (`KismetStringLibrary.Concat_StrStr` "Bot" (`KismetStringLibrary.Conv_IntToString` IdNum) "," (`KismetStringLibrary.Conv_IntToString` IdNum) "," (`KismetStringLibrary.Conv_DoubleToString` Mu) "," (`KismetStringLibrary.Conv_DoubleToString` Sigma))))

(fn `BotStatsVarToStringTS`
  (params (BotID :type Integer) (InGame :type Boolean) (GamesPlayed :type Integer) (Mu :type "Float (double-precision)") (Sigma :type "Float (double-precision)"))
  (returns (NewParam :type String))
  (return (`KismetStringLibrary.Concat_StrStr` "Bot" (`KismetStringLibrary.Conv_IntToString` BotID) "," (`KismetStringLibrary.Conv_IntToString` BotID) "," "FALSE" "," (`KismetStringLibrary.Conv_IntToString` GamesPlayed) "," (`KismetStringLibrary.Conv_DoubleToString` Mu) "," (`KismetStringLibrary.Conv_DoubleToString` Sigma))))

(fn `ServerStatsVarToString`
  (params (IDNum :type Integer) (InGame :type Boolean) (GamesPlayed :type Integer) (SkillRating :type "Float (double-precision)"))
  (returns (OutString :type String))
  (return (`KismetStringLibrary.Concat_StrStr` "Bot" (`KismetStringLibrary.Conv_IntToString` IDNum) "," (`KismetStringLibrary.Conv_IntToString` IDNum) "," "FALSE" "," (`KismetStringLibrary.Conv_IntToString` GamesPlayed) "," (`KismetStringLibrary.Conv_DoubleToString` SkillRating))))

(fn `ServerVarToString`
  (params (InputString :type String))
  (returns (IdNum :type Integer) (InGame :type Boolean) (GamesPlayed :type Integer) (SkillRating :type "Float (double-precision)"))
  (bind _returnvalue (`KismetStringLibrary.ParseIntoArray` InputString ","))
  (return (`KismetStringLibrary.Conv_StringToInt` (`|GetArrayItem` _returnvalue 1)) false (`KismetStringLibrary.Conv_StringToInt` (`|GetArrayItem` _returnvalue 3)) (`KismetStringLibrary.Conv_StringToDouble` (`|GetArrayItem` _returnvalue 4))))

(fn `UserConstructionScript`)