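; Bot_AI_BP is the AI controller for bots, running the Bot_BT behavior tree on BeginPlay.
; Perception updates for Bot_BP actors with a different TeamTag than the controlled pawn set the TargetActor blackboard key and focus on that actor.
; Losing perception starts a one-second timer that clears the target and focus, which a fresh successful sensing cancels.
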(event `self.ReceiveBeginPlay`
  (`self.RunBehaviorTree` "/Game/Bot_BT.Bot_BT"))

(event `self.AIPerception.OnTargetPerceptionUpdated`
  (params (Actor :type "Actor Object Reference") (Stimulus :type "AIStimulus Structure"))
  (bind _sensedactor (`self.SensedActor`))
  (bind _asbot_bp (cast `/Game/Bot_BP` Actor))
  (`/Engine/EditorBlueprintResources/StandardMacros.IsValid` _asbot_bp
    (:`Is Valid`
      (bind _asbot_bp_2 (cast `/Game/Bot_BP` (`self.K2_GetPawn` self)))
      (set `self.SensedActor` Actor)
      (if (!= (`/Game/Bot_BP.TeamTag` _asbot_bp) (`/Game/Bot_BP.TeamTag` _asbot_bp_2))
        (if (`.bSuccessfullySensed` (break `AIStimulus` Stimulus))
          (`BlackboardComponent.SetValueAsObject` (`self.Blackboard`) "TargetActor" _sensedactor)
          (`self.K2_SetFocus` _sensedactor)
          (`KismetSystemLibrary.K2_ClearAndInvalidateTimerHandle` (`self.LoseTargetTimer`))
          (else
            (bind _returnvalue (`KismetSystemLibrary.K2_SetTimerDelegate` (delegate `LoseTarget`) 1.0))
            (set `self.LoseTargetTimer` _returnvalue)))))))

(event `LoseTarget`
  (`BlackboardComponent.SetValueAsObject` (`self.Blackboard`) "TargetActor" null)
  (`self.K2_ClearFocus`))

(fn `UserConstructionScript`)