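; AI bot for a red-versus-blue team shooter, with team tag and material set at construction or by event.
; FireBullet waits a reaction delay, then line-traces toward the controller's focus actor with random inaccuracy, applying damage and effects.
; Damage feeds AI sense reporting; death clears the killer bot's target and notifies a controller to check remaining enemies.
; Dead bots are teleported away with brain logic stopped, then respawned by teleporting back and restarting it.
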(event `FireBullet`
  (bind _reverseaccuracy (`self.ReverseAccuracy`))
  (bind _accuracy (`self.Accuracy`))
  (bind _returnvalue (`AIController.GetFocusActor` (`AIBlueprintHelperLibrary.GetAIController` self)))
  (`KismetSystemLibrary.Delay` (`self.ReactionTime`))
  (`/Engine/EditorBlueprintResources/StandardMacros.IsValid` _returnvalue
    (:`Is Valid`
      (bind (_outhit _returnvalue_2) (`KismetSystemLibrary.LineTraceSingle` :`Start` (`SceneComponent.K2_GetComponentLocation` (`self.Gun`)) :`End` (`KismetMathLibrary.GreaterGreater_VectorRotator` (`self.K2_GetActorLocation` _returnvalue) (`KismetMathLibrary.MakeRotator` (`KismetMathLibrary.RandomFloatInRange` _reverseaccuracy _accuracy) (`KismetMathLibrary.RandomFloatInRange` _reverseaccuracy _accuracy))) :`TraceChannel` "TraceTypeQuery2" :`DrawDebugType` "ForOneFrame"))
      (bind (_bblockinghit _binitialoverlap _time _distance _location _impactpoint _normal _impactnormal _physmat _hitactor) (`GameplayStatics.BreakHitResult` _outhit))
      (`GameplayStatics.ApplyPointDamage` _hitactor 0.5 _impactnormal _outhit null self)
      (bind (_bblockinghit_2 _binitialoverlap_2 _time_2 _distance_2 _location_2 _impactpoint_2 _normal_2 _impactnormal_2 _physmat_2 _hitactor_2 _hitcomponent _hitbonename _bonename _hititem _elementindex _faceindex _tracestart _traceend) (`GameplayStatics.BreakHitResult` _outhit))
      (`NiagaraFunctionLibrary.SpawnSystemAtLocation` null _tracestart (`KismetMathLibrary.FindLookAtRotation` _tracestart _traceend))
      (`GameplayStatics.PlaySoundAtLocation` "/Game/FPWeapon/Audio/FireCue.FireCue" (`self.K2_GetActorLocation`) (struct) 1.0 1.0 0.0 null null null null)
      (if _returnvalue_2
        (`NiagaraFunctionLibrary.SpawnSystemAtLocation` null _location (`KismetMathLibrary.Conv_VectorToRotator` _impactpoint))))))

(event `self.ReceiveAnyDamage`
  (params (Damage :type "Float (single-precision)") (DamageType :type "DamageType Object Reference") (InstigatedBy :type "Controller Object Reference") (DamageCauser :type "Actor Object Reference"))
  (bind _output_get (set `self.Health` (- (`self.Health`) Damage)))
  (if (<= _output_get 0.0)
    (`self.EnemyDeath`)
    (`self.Died`)
    (set `self.Isdead_0` true)
    (`SpawnController.CheckEnemysLeft` (`self.ReportToController`) (== (`self.TeamTag`) (struct :`TagName` "Team.BlueTeam")))
    (else
      (`AISense_Damage.ReportDamageEvent` self DamageCauser Damage (`self.K2_GetActorLocation`)))))

(event `EnemyDeath`
  (bind _asbot_bp (cast `/Game/Bot_BP` (stale `self.ReceiveAnyDamage` DamageCauser)))
  (bind _returnvalue (`AIBlueprintHelperLibrary.GetAIController` _asbot_bp))
  (`BlackboardComponent.SetValueAsObject` (`AIBlueprintHelperLibrary.GetBlackboard` _returnvalue) "TargetActor" null)
  (`AIController.K2_ClearFocus` _returnvalue)
  (`self.KilledEnemy` _asbot_bp)
  (`self.K2_SetActorLocation` self (-1000.0 -1000.0 -100.0) false true)
  (`BrainComponent.StopLogic` (`AIController.BrainComponent` (`AIBlueprintHelperLibrary.GetAIController` self)) "Dead"))

(event `self.RespawnRedBot`
  (params (SpawnPos :type "Vector Structure"))
  (`self.K2_SetActorLocation` SpawnPos false true)
  (`BrainComponent.StartLogic` (`AIController.BrainComponent` (`AIBlueprintHelperLibrary.GetAIController` self)) :!label _label))

(event `self.RespawnBlueBot`
  (params (SpawnPos :type "Vector Structure"))
  (`self.K2_SetActorLocation` SpawnPos false true)
  (goto _label))

(event `self.SetBlueTeam`
  (set `self.TeamTag` (struct :`TagName` "Team.BlueTeam"))
  (`PrimitiveComponent.SetMaterial` (`self.Mesh`) 0 "/Game/LevelPrototyping/Materials/MI_Solid_Blue.MI_Solid_Blue"))

(event `self.SetRedTeam`
  (set `self.TeamTag` (struct :`TagName` "Team.RedTeam"))
  (`PrimitiveComponent.SetMaterial` (`self.Mesh`) 0 "/Game/FPWeapon/Materials/FirstPersonProjectileMaterial.FirstPersonProjectileMaterial"))

(fn `UserConstructionScript`
  (bind _teamtag (`self.TeamTag`))
  (bind _mesh (`self.Mesh`))
  (`BlueprintGameplayTagLibrary.AddGameplayTag` (`self.ActorTagContainer`) _teamtag)
  (if (== (struct :`TagName` "Team.BlueTeam") _teamtag)
    (`PrimitiveComponent.SetMaterial` _mesh 0 "/Game/LevelPrototyping/Materials/MI_Solid_Blue.MI_Solid_Blue")
    (else
      (`PrimitiveComponent.SetMaterial` _mesh 0 "/Game/FPWeapon/Materials/FirstPersonProjectileMaterial.FirstPersonProjectileMaterial"))))